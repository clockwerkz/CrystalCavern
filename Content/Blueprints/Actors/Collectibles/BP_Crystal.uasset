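; BP_Crystal is a collectible crystal actor that plays a pickup animation when the player overlaps it, then destroys itself.
; On overlap it caches its location, scale and light intensity, then plays CollectionTimeline.
; Separate timeline tracks drive lerps that pull it toward the player pawn's live position, shrink it to zero and fade out CrystalLight.
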(event `self.ReceiveActorBeginOverlap`
  (params (OtherActor :type "Actor Object Reference"))
  (`/Game/Blueprints/Libraries/CC_MacroLibrary.isPlayer` OtherActor
    (:`isPlayer`
      (`self.StoreStartingValues`)
      (bind (_direction _collection_progress _scale_progress _light_dim_progress) (`Timeline|CollectionTimeline`)
        (:`Update`
          (`self.MoveToPlayer` _collection_progress)
          (`self.ScaleCrystal` _scale_progress)
          (`self.AdjustLight` _light_dim_progress))
        (:`Finished`
          (`self.K2_DestroyActor`))))))

(fn `AdjustLight`
  (params (Alpha :type "Float (double-precision)"))
  (`LightComponent.SetIntensity` (`self.CrystalLight`) (`KismetMathLibrary.Lerp` (`self.StartingLightIntensity`) 0.0 Alpha)))

(fn `MoveToPlayer`
  (params (Alpha :type "Float (double-precision)"))
  (`self.K2_SetActorLocation` (`KismetMathLibrary.VLerp` (`self.LerpStartLocation`) (`self.K2_GetActorLocation` (`GameplayStatics.GetPlayerPawn` 0)) Alpha)))

(fn `ScaleCrystal`
  (params (Alpha :type "Float (double-precision)"))
  (`self.SetActorScale3D` (`KismetMathLibrary.VLerp` (`self.StartScale`) (0.0 0.0 0.0) Alpha)))

(fn `StoreStartingValues`
  (set `self.LerpStartLocation` (`self.K2_GetActorLocation`))
  (set `self.StartScale` (`self.GetActorScale3D`))
  (set `self.StartingLightIntensity` (`LightComponentBase.Intensity` (`self.CrystalLight`))))

(fn `UserConstructionScript`)