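; BP_Cannon is an enemy cannon actor that fires repeatedly on its own from BeginPlay, without any targeting.
; Each cycle waits for the fire-rate delay, then spawns an actor at the projectile spawn point's location and rotation with a configurable scale.
; CannonTimeline then animates the barrel along its local Y axis, and its Cannon Fired event loops back to the delay, so no Tick is used.
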(event `self.ReceiveBeginPlay`
  (`KismetSystemLibrary.Delay` (`self.Cannon Fire Rate`) :!label _label)
  (`self.Spawn Projectile`)
  (bind (_direction _fire_sequence) (`Timeline|Cannon Timeline` :!via `PlayFromStart`)
    (:`Update`
      (`self.Move Cannon Barrel` _fire_sequence))
    (:`Cannon Fired`
      (goto _label))))

(fn `Move Cannon Barrel`
  (params (`Cannon Barrel Y Location` :type "Float (double-precision)"))
  (`SceneComponent.K2_SetRelativeLocation` (`self.Cannon Barrel`) (`KismetMathLibrary.MakeVector` 0.0 `Cannon Barrel Y Location`) false false))

(fn `Spawn Projectile`
  (bind (_returnvalue_location _returnvalue_rotation) (`KismetMathLibrary.BreakTransform` (`SceneComponent.K2_GetComponentToWorld` (`self.ProjectileSpawnPoint`))))
  (`|SpawnActorFromClass` "/Game/Blueprints/Actors/Projectiles/BR_Projectile.BR_Projectile_C" (`KismetMathLibrary.MakeTransform` _returnvalue_location _returnvalue_rotation (`KismetMathLibrary.Conv_DoubleToVector` (`self.Projectile Scale`))) "Undefined" "OverrideRootScale" null null))

(fn `UserConstructionScript`)